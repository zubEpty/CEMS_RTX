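; Exhibitor Blueprint that fetches the current exhibitor's profile from a remote web API when play begins.
; It reads a bearer token from the TokenPasser game instance and sends an authorized VaRest GET request to the exhibitors/me endpoint.
; On completion it prints the company name from the nested user object in the JSON response, and on failure it prints an error message.
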(event Custom|ResponseFailure
  (params (Request :type Va%20Rest%20Request%20JSON%20Object%20Reference))
  (Development|PrintString "Response failed"))

(event Custom|ResponseProfile
  (params (Request :type Va%20Rest%20Request%20JSON%20Object%20Reference))
  (bind _returnvalue (Class|VaRestJsonValue|AsObject (Class|VaRestJsonObject|GetField (Class|VaRestRequestJSON|GetResponseObject Request) "message")))
  (bind _returnvalue_2 (Class|VaRestJsonValue|AsObject (Class|VaRestJsonObject|GetField _returnvalue "user")))
  (Development|PrintString (Class|VaRestJsonObject|GetStringField _returnvalue_2 "company_name")))

(event EventBeginPlay
  (bind _astoken_passer (Utilities|Casting|CastToTokenPasser (Game|GetGameInstance)))
  (bind _output_get (Variables|Default|SetToken (Variables|/Game/Blueprints/TokenPasser.TokenPasser_C|GetBearerToken _astoken_passer)))
  (bind _returnvalue (Class|VaRestSubsystem|ConstructVaRestRequestExt (|VaRestSubsystem) "GET" "x_www_form_urlencoded_url"))
  (Class|VaRestRequestJSON|SetHeader _returnvalue "Authorization" (Utilities|String|Append "Bearer " _output_get))
  (EventDispatchers|BindEventtoOnRequestComplete _returnvalue (delegate Custom|ResponseProfile))
  (EventDispatchers|BindEventtoOnRequestFail _returnvalue (delegate Custom|ResponseFailure))
  (Class|VaRestRequestJSON|ProcessURL _returnvalue "https://api-ve.studio-23.xyz/exhibitors/me"))

(fn ConstructionScript)