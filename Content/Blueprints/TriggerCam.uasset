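; TriggerCam is a clickable camera trigger that shows a hand cursor on hover and glides the player's pawn to its CameraToFind when clicked.
; Timelines lerp the pawn's current location toward the target, and TimelineEvent does the same for a passed-in camera.
; When flagged IsBoothCam, an overlap opens the BoothUI widget.
; View-target blend, rotation lerp and hide nodes are unconnected, so only location changes.
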(event Custom|TimelineEvent
  (params (BPCamera :type Camera%20Actor%20Object%20Reference))
  (bind _returnvalue (Game|GetPlayerController 0))
  (bind _returnvalue_2 (Pawn|GetControlledPawn _returnvalue))
  (bind _alpha (Timeline|Timeline_2 PlayFromStart)
    (:Update
      (Transformation|SetActorLocation _returnvalue_2 (Math|Vector|Lerp(Vector) (Transformation|GetActorLocation _returnvalue_2) (Transformation|GetActorLocation BPCamera) _alpha) false false))))

(event MouseInput|EventActorBeginCursorOver
  ;[1 1 1] Cursor Icon Change
  (Variables|/Script/Engine.PlayerController|SetCurrentMouseCursor (Game|GetPlayerController 0) "Hand"))

(event MouseInput|EventActorEndCursorOver
  ;[1 1 1] Cursor Icon Change
  (Variables|/Script/Engine.PlayerController|SetCurrentMouseCursor (Game|GetPlayerController 0) "Default"))

(event MouseInput|EventActorOnClicked
  (params (ButtonPressed :type Key%20Structure :default "None"))
  (bind _returnvalue (Game|GetPlayerController 0))
  (bind _returnvalue_2 (Pawn|GetControlledPawn _returnvalue))
  ;[1 1 1] Camera Blend with Controller
  (bind _asplayer_controller (Utilities|Casting|CastToPlayerController (Game|GetPlayerController 0)))
  (if (Utilities|IsValid _asplayer_controller)
    ;[1 1 1] Player Smooth Transition
    (bind _alpha (Timeline|Timeline_0 Play)
      (:Update
        (Transformation|SetActorLocation _returnvalue_2 (Math|Vector|Lerp(Vector) (Transformation|GetActorLocation _returnvalue_2) (Transformation|GetActorLocation (Variables|Default|GetCameraToFind)) _alpha) false false)))))

(event Collision|EventActorBeginOverlap
  (params (OtherActor :type Actor%20Object%20Reference))
  (if (Variables|Default|GetisBoothCam)
    (Utilities|IsValid OtherActor
      (:Is%20Valid
        (bind _returnvalue (UserInterface|CreateWidget "/Game/UI/BoothUI.BoothUI_C"))
        (UserInterface|Viewport|AddtoViewport _returnvalue 0)))
    (else
      (Utilities|IsValid OtherActor))))

(fn ConstructionScript)