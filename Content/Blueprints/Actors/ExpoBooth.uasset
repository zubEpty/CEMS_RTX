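; Expo booth actor that fills its four banner meshes with ad images fetched from a web API.
; Shortly after BeginPlay it looks up its entry in the BoothController by Id and sends a VaRest GET for that booth's data.
; The response's image list drives chained DownloadImage calls, each started without waiting for the previous download to finish.
; Each banner gets a dynamic DefaultAd material, whose texture is set when its download succeeds.
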(event Custom|Response
  (params (Request :type Va%20Rest%20Request%20JSON%20Object%20Reference))
  (bind _topbanner (Variables|Default|GetTopBanner))
  (bind _banner (Variables|Default|GetBanner))
  (bind _downbanner (Variables|Default|GetDownBanner))
  (bind _longbanner (Variables|Default|GetLongBanner))
  ;[1 1 1] Get Json Data
  (bind _returnvalue (Class|VaRestJsonValue|AsObject (Class|VaRestJsonObject|GetField (Class|VaRestRequestJSON|GetResponseObject Request) "message")))
  (bind _returnvalue_2 (Class|VaRestJsonValue|AsObject (Utilities|Array|Get(acopy) (Class|VaRestJsonObject|GetArrayField _returnvalue "images"))))
  (bind _texture (|DownloadImage (Class|VaRestJsonObject|GetStringField _returnvalue_2 "file_name"))
    (:then
      ;[1 1 1] Load Texture into Material
      (bind _returnvalue_3 (Rendering|Material|CreateDynamicMaterialInstance _topbanner 0 "/Game/Banners/DefaultAd.DefaultAd" "None" :!class /Script/Engine.PrimitiveComponent))
      (Rendering|Material|SetMaterial _topbanner 0 _returnvalue_3)
      (bind _returnvalue_4 (Class|VaRestJsonValue|AsObject (Utilities|Array|Get(acopy) (Class|VaRestJsonObject|GetArrayField _returnvalue "images") 1)))
      (bind _texture_2 (|DownloadImage (Class|VaRestJsonObject|GetStringField _returnvalue_4 "file_name"))
        (:then
          ;[1 1 1] Load Texture into Material
          (bind _returnvalue_5 (Rendering|Material|CreateDynamicMaterialInstance _banner 0 "/Game/Banners/DefaultAd.DefaultAd" "None" :!class /Script/Engine.PrimitiveComponent))
          (Rendering|Material|SetMaterial _banner 0 _returnvalue_5)
          (bind _returnvalue_6 (Class|VaRestJsonValue|AsObject (Utilities|Array|Get(acopy) (Class|VaRestJsonObject|GetArrayField _returnvalue "images") 2)))
          (bind _texture_3 (|DownloadImage (Class|VaRestJsonObject|GetStringField _returnvalue_6 "file_name"))
            (:then
              ;[1 1 1] Load Texture into Material
              (bind _returnvalue_7 (Rendering|Material|CreateDynamicMaterialInstance _downbanner 0 "/Game/Banners/DefaultAd.DefaultAd" "None" :!class /Script/Engine.PrimitiveComponent))
              (Rendering|Material|SetMaterial _downbanner 0 _returnvalue_7)
              (bind _returnvalue_8 (Class|VaRestJsonValue|AsObject (Utilities|Array|Get(acopy) (Class|VaRestJsonObject|GetArrayField _returnvalue "images") 3)))
              (bind _texture_4 (|DownloadImage (Class|VaRestJsonObject|GetStringField _returnvalue_8 "file_name"))
                (:then
                  ;[1 1 1] Load Texture into Material
                  (bind _returnvalue_9 (Rendering|Material|CreateDynamicMaterialInstance _longbanner 0 "/Game/Banners/DefaultAd.DefaultAd" "None" :!class /Script/Engine.PrimitiveComponent))
                  (Rendering|Material|SetMaterial _longbanner 0 _returnvalue_9))
                (:OnSuccess
                  (Rendering|Material|SetTextureParameterValue _returnvalue_9 "DefaultBase" _texture_4))
                (:OnFail
                  (Development|PrintString "URL error"))))
            (:OnSuccess
              (Rendering|Material|SetTextureParameterValue _returnvalue_7 "DefaultBase" _texture_3))
            (:OnFail
              (Development|PrintString "URL error"))))
        (:OnSuccess
          (Rendering|Material|SetTextureParameterValue _returnvalue_5 "DefaultBase" _texture_2))
        (:OnFail
          (Development|PrintString "URL error"))))
    (:OnSuccess
      (Rendering|Material|SetTextureParameterValue _returnvalue_3 "DefaultBase" _texture))
    (:OnFail
      (Development|PrintString "URL error"))))

(event EventBeginPlay
  (bind _returnvalue (|VaRestSubsystem))
  (Utilities|FlowControl|Delay 2.0)
  (bind _returnvalue_2 (Actor|GetActorOfClass "/Game/Blueprints/Actors/BoothController.BoothController_C"))
  ;[1 1 1] Get Json Data
  (bind _returnvalue_3 (Class|VaRestSubsystem|ConstructVaRestJsonObject _returnvalue))
  (Class|VaRestSubsystem|CallURL _returnvalue (Utilities|String|Append (Variables|Default|GetURL) (Utilities|String|ToString(Integer) (Utilities|Array|Get(acopy) (Variables|/Game/Blueprints/Actors/BoothController.BoothController_C|GetBooth _returnvalue_2) (Variables|Default|GetId)))) "GET" "x_www_form_urlencoded_url" _returnvalue_3 (delegate Custom|Response)))

(fn ConstructionScript)