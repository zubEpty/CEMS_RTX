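; BoothController is an actor that retrieves the booth IDs of exhibitors in a conference exhibition hall.
; On BeginPlay it sends a VaRest GET request to a hard-coded exhibitor-list endpoint for hall 10.
; The response callback walks the returned "message" array, adds each nested booth ID to the Booth variable and prints a debug message per entry.
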(event Custom|Response
  (params (Request :type Va%20Rest%20Request%20JSON%20Object%20Reference))
  (for _array_element (Class|VaRestJsonObject|GetArrayField (Class|VaRestRequestJSON|GetResponseObject Request) "message")
    (bind _returnvalue (Class|VaRestJsonValue|AsObject _array_element))
    (bind _returnvalue_2 (Class|VaRestJsonValue|AsObject (Class|VaRestJsonObject|GetField _returnvalue "booth")))
    (Utilities|Array|Add (Variables|Default|GetBooth) (Class|VaRestJsonObject|GetIntegerField _returnvalue_2 "id"))
    (Development|PrintString "List updated")))

(event EventBeginPlay
  (bind _returnvalue (|VaRestSubsystem))
  (bind _returnvalue_2 (Class|VaRestSubsystem|ConstructVaRestJsonObject _returnvalue))
  (Class|VaRestSubsystem|CallURL _returnvalue "https://api-ve.studio-23.xyz/conference-hall/exhibition-hall/10/exhibitor-list" "GET" "x_www_form_urlencoded_url" _returnvalue_2 (delegate Custom|Response)))

(fn ConstructionScript)