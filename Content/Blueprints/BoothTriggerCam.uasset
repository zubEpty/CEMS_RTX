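; Clickable booth camera trigger that moves the player to a booth viewpoint and shows that booth's web-sourced content.
; Hover switches the cursor to a hand; a click or TimelineEvent lerps the pawn's location to a camera actor via timelines.
; Overlap sends a VaRest GET using an ID from BoothController, then fills a new BoothUI with video, document and product fields.
; View-target blend and rotation logic are disconnected.
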(event Custom|TimelineEvent
  (params (BPCamera :type Camera%20Actor%20Object%20Reference))
  (bind _returnvalue (Game|GetPlayerController 0))
  (bind _returnvalue_2 (Pawn|GetControlledPawn _returnvalue))
  (bind _alpha (Timeline|Timeline_2 PlayFromStart)
    (:Update
      (Transformation|SetActorLocation _returnvalue_2 (Math|Vector|Lerp(Vector) (Transformation|GetActorLocation _returnvalue_2) (Transformation|GetActorLocation BPCamera) _alpha) false false))))

(event Custom|Response
  (params (Request :type Va%20Rest%20Request%20JSON%20Object%20Reference))
  ;[1 1 1] Get Json Data
  (bind _returnvalue (Class|VaRestJsonValue|AsObject (Class|VaRestJsonObject|GetField (Class|VaRestRequestJSON|GetResponseObject Request) "message")))
  (bind _returnvalue_2 (Class|VaRestJsonValue|AsObject (Utilities|Array|Get(acopy) (Class|VaRestJsonObject|GetArrayField _returnvalue "videos"))))
  (bind _returnvalue_3 (UserInterface|CreateWidget "/Game/UI/BoothUI.BoothUI_C"))
  (UserInterface|Viewport|AddtoViewport _returnvalue_3 0)
  (Rendering|Components|TextRender|SetText (Variables|/Game/UI/BoothUI.BoothUI_C|GetURL _returnvalue_3) (Utilities|Text|ToText(String) (Class|VaRestJsonObject|GetStringField _returnvalue_2 "file_name")))
  (bind _returnvalue_4 (Class|VaRestJsonValue|AsObject (Utilities|Array|Get(acopy) (Class|VaRestJsonObject|GetArrayField _returnvalue "videos") 1)))
  (Rendering|Components|TextRender|SetText (Variables|/Game/UI/BoothUI.BoothUI_C|GetURL_1 _returnvalue_3) (Utilities|Text|ToText(String) (Class|VaRestJsonObject|GetStringField _returnvalue_4 "file_name")))
  (bind _returnvalue_5 (Class|VaRestJsonValue|AsObject (Utilities|Array|Get(acopy) (Class|VaRestJsonObject|GetArrayField _returnvalue "documents"))))
  (Variables|/Game/UI/BoothUI.BoothUI_C|Setdocument_url _returnvalue_3 (Class|VaRestJsonObject|GetStringField _returnvalue_5 "file_name"))
  (bind _returnvalue_6 (Class|VaRestJsonValue|AsObject (Utilities|Array|Get(acopy) (Class|VaRestJsonObject|GetArrayField _returnvalue "products"))))
  (Variables|/Game/UI/BoothUI.BoothUI_C|Setimage_url _returnvalue_3 (Class|VaRestJsonObject|GetStringField _returnvalue_6 "image"))
  (Rendering|Components|TextRender|SetText (Variables|/Game/UI/BoothUI.BoothUI_C|GetProduct_Title _returnvalue_3) (Utilities|Text|ToText(String) (Class|VaRestJsonObject|GetStringField _returnvalue_6 "title")))
  (Rendering|Components|TextRender|SetText (Variables|/Game/UI/BoothUI.BoothUI_C|GetDescription_box _returnvalue_3) (Utilities|Text|ToText(String) (Class|VaRestJsonObject|GetStringField _returnvalue_6 "description")))
  (Rendering|Components|TextRender|SetText (Variables|/Game/UI/BoothUI.BoothUI_C|GetKeyfeatures-1 _returnvalue_3) (Utilities|Text|ToText(String) (Utilities|Array|Get(acopy) (Class|VaRestJsonObject|GetStringArrayField _returnvalue_6 "key_features"))))
  (Rendering|Components|TextRender|SetText (Variables|/Game/UI/BoothUI.BoothUI_C|GetKeyfeature-2 _returnvalue_3) (Utilities|Text|ToText(String) (Utilities|Array|Get(acopy) (Class|VaRestJsonObject|GetStringArrayField _returnvalue_6 "key_features") 1))))

(event MouseInput|EventActorBeginCursorOver
  ;[1 1 1] Cursor Icon Change
  (Variables|/Script/Engine.PlayerController|SetCurrentMouseCursor (Game|GetPlayerController 0) "Hand"))

(event MouseInput|EventActorEndCursorOver
  ;[1 1 1] Cursor Icon Change
  (Variables|/Script/Engine.PlayerController|SetCurrentMouseCursor (Game|GetPlayerController 0) "Default"))

(event MouseInput|EventActorOnClicked
  (params (ButtonPressed :type Key%20Structure :default "None"))
  (bind _returnvalue (Game|GetPlayerController 0))
  (bind _returnvalue_2 (Pawn|GetControlledPawn _returnvalue))
  ;[1 1 1] Camera Blend with Controller
  (bind _asplayer_controller (Utilities|Casting|CastToPlayerController (Game|GetPlayerController 0)))
  (if (Utilities|IsValid _asplayer_controller)
    ;[1 1 1] Player Smooth Transition
    (bind _alpha (Timeline|Timeline_0 Play)
      (:Update
        (Transformation|SetActorLocation _returnvalue_2 (Math|Vector|Lerp(Vector) (Transformation|GetActorLocation _returnvalue_2) (Transformation|GetActorLocation (Variables|Default|GetCameraToFind)) _alpha) false false)))))

(event Collision|EventActorBeginOverlap
  (params (OtherActor :type Actor%20Object%20Reference))
  (bind _returnvalue (|VaRestSubsystem))
  (bind _returnvalue_2 (Actor|GetActorOfClass "/Game/Blueprints/Actors/BoothController.BoothController_C"))
  ;[1 1 1] Get Json Data
  (bind _returnvalue_3 (Class|VaRestSubsystem|ConstructVaRestJsonObject _returnvalue))
  (Class|VaRestSubsystem|CallURL _returnvalue (Utilities|String|Append "https://api-ve.studio-23.xyz/booth/" (Utilities|String|ToString(Integer) (Utilities|Array|Get(acopy) (Variables|/Game/Blueprints/Actors/BoothController.BoothController_C|GetBooth _returnvalue_2) (Variables|/Game/Blueprints/Actors/ExpoBooth.ExpoBooth_C|GetId (Variables|Default|GetBooth))))) "GET" "x_www_form_urlencoded_url" _returnvalue_3 (delegate Custom|Response)))

(fn ConstructionScript)